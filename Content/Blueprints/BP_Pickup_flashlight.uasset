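; Flashlight pickup actor that blinks in the world until the player collects it.
; Tick runs through a delay into a flip-flop that switches its spot and point lights off and on.
; Interact works only once PickupKey has set HasBattery; it then adds a flashlight component to the first-person character and destroys the pickup.
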(event EventPickupKey
  (Variables|Default|SethasBattery true))

(event EventTick
  (params (DeltaSeconds :type Float%20%28single-precision%29))
  (bind _spotlight (Variables|Default|GetSpotLight))
  ;[1 1 1] Flickering
  (Utilities|FlowControl|Delay 1.0)
  (Utilities|FlowControl|FlipFlop
    (:A
      (Rendering|Components|Light|SetIntensity _spotlight 0.0))
    (:B
      (Rendering|Components|Light|SetIntensity _spotlight 1e+05))))

(event EventInteract
  (if (Variables|Default|GethasBattery)
    (bind _asbp_first_person_character (Utilities|Casting|CastToBP_FirstPersonCharacter (Game|GetPlayerCharacter 0)))
    (bind _output_get (Variables|Default|SetFirst%20Person%20Character%20Reference _asbp_first_person_character))
    (AddComponent|AddBPFlashlightComponent _output_get false)
    (Actor|DestroyActor)))

(fn ConstructionScript)