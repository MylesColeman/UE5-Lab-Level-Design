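; BP_Note is an interactable note actor that switches the NoteInteract flag on the first-person character.
; It caches the player character on BeginPlay, and each Interact toggles that flag after a short delay.
; Overlap events track whether something is inside the note's range, and Tick forces the flag false whenever nothing is marked as overlapping, so walking away clears it.
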(event Collision|EventActorEndOverlap
  (params (OtherActor :type Actor%20Object%20Reference))
  ;[1 1 1] Walked away?
  (Variables|Default|Setoverlapping false))

(event EventBeginPlay
  ;[1 1 1] Interacted?
  (bind _asbp_first_person_character (Utilities|Casting|CastToBP_FirstPersonCharacter (Game|GetPlayerCharacter 0))))

(event EventInteract
  ;[1 1 1] Interacted?
  (Utilities|FlowControl|Delay 0.1)
  (if (Variables|/Game/FirstPerson/Blueprints/BP_FirstPersonCharacter.BP_FirstPersonCharacter_C|GetnoteInteract (stale EventBeginPlay _asbp_first_person_character))
    (Variables|/Game/FirstPerson/Blueprints/BP_FirstPersonCharacter.BP_FirstPersonCharacter_C|SetnoteInteract (stale EventBeginPlay _asbp_first_person_character) false)
    (else
      (Variables|/Game/FirstPerson/Blueprints/BP_FirstPersonCharacter.BP_FirstPersonCharacter_C|SetnoteInteract (stale EventBeginPlay _asbp_first_person_character) true))))

(event Collision|EventActorBeginOverlap
  (params (OtherActor :type Actor%20Object%20Reference))
  ;[1 1 1] Walked away?
  (Variables|Default|Setoverlapping true))

(event EventTick
  (params (DeltaSeconds :type Float%20%28single-precision%29))
  ;[1 1 1] Walked away?
  (if (not (Variables|Default|Getoverlapping))
    (Variables|/Game/FirstPerson/Blueprints/BP_FirstPersonCharacter.BP_FirstPersonCharacter_C|SetnoteInteract (stale EventBeginPlay _asbp_first_person_character) false)))

(fn ConstructionScript)