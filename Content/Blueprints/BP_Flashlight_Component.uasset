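; BP_Flashlight_Component equips the first-person character with a flashlight and a battery level display.
; On BeginPlay it casts its owner to BP_FirstPersonCharacter, snaps itself to the character's flashlight scene component and sets HasTorch.
; It also creates a scaled plane mesh at runtime with the battery level material and attaches it to the character's display component at FlashlightSocket, keeping relative scale.
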(event EventBeginPlay
  (bind _asbp_first_person_character (Utilities|Casting|CastToBP_FirstPersonCharacter (Components|GetOwner)))
  (bind _output_get (Variables|Default|SetFirst%20Person%20Char _asbp_first_person_character))
  (Transformation|AttachComponentToComponent (Variables|/Game/FirstPerson/Blueprints/BP_FirstPersonCharacter.BP_FirstPersonCharacter_C|GetScene_Flashlight _output_get) " " "SnapToTarget" "SnapToTarget" "SnapToTarget" true)
  (Variables|/Game/FirstPerson/Blueprints/BP_FirstPersonCharacter.BP_FirstPersonCharacter_C|SethasTorch _output_get true)
  (bind _returnvalue (Game|AddComponentbyClass _output_get "/Script/Engine.StaticMeshComponent" false (Math|Transform|MakeTransform "0, 0, 0" "0.000000,0.000000,90.000000" "0.040000,0.057500,1.000000")))
  (Variables|Default|SetDisplayPlane _returnvalue)
  (Components|StaticMesh|SetStaticMesh _returnvalue "/Game/StarterContent/Shapes/Shape_Plane.Shape_Plane")
  (Rendering|Material|SetMaterial _returnvalue 0 "/Game/Assets/M_BatteryLevel.M_BatteryLevel")
  (Transformation|AttachComponentToComponent _returnvalue (Variables|/Game/FirstPerson/Blueprints/BP_FirstPersonCharacter.BP_FirstPersonCharacter_C|GetScene_Display (Variables|Default|GetFirst%20Person%20Char)) "FlashlightSocket " "SnapToTarget" "SnapToTarget" "KeepRelative" true))